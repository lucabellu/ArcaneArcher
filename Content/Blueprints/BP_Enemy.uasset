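; BP_Enemy is an enemy actor that is destroyed by any damage, regardless of the amount.
; On taking damage it prints the value, then destroys itself after a short delay.
; On BeginPlay it caches the first-person player character and binds to its own OnDestroyed event, which removes it from the array in that character's EnemyCounter.
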(event Custom|RemoveFromArray
  (params (DestroyedActor :type Actor%20Object%20Reference))
  (Default|RemoveEnemyfromArray (Variables|/Game/FirstPerson/Blueprints/BP_FirstPersonCharacter.BP_FirstPersonCharacter_C|GetEnemyCounter (stale EventBeginPlay _asbp_first_person_character)) self))

(event EventBeginPlay
  (bind _asbp_first_person_character (Utilities|Casting|CastToBP_FirstPersonCharacter (Game|GetPlayerCharacter 0)))
  (Game|BindEventtoOnDestroyed (delegate Custom|RemoveFromArray)))

(event Game|Damage|EventAnyDamage
  (params (Damage :type Float%20%28single-precision%29) (DamageType :type Damage%20Type%20Object%20Reference) (InstigatedBy :type Controller%20Object%20Reference) (DamageCauser :type Actor%20Object%20Reference))
  (Development|PrintString (Utilities|String|ToString(Float) Damage))
  (Utilities|FlowControl|Delay 0.2)
  (Actor|DestroyActor))

(fn ConstructionScript)