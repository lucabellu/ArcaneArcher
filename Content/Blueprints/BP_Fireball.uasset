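; BP_Fireball is a fireball actor that explodes on hit, damaging nearby objects and knocking the player away from the blast.
; On hit it plays the explosion sound at the player's location and spawns a scaled-up particle effect at the impact point.
; A sphere trace over WorldDynamic objects applies flat damage and flags any Player-tagged actor.
; A flagged player is launched away from the impact, and the fireball destroys itself.
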(event Collision|EventHit
  (params (MyComp :type Primitive%20Component%20Object%20Reference) (Other :type Actor%20Object%20Reference) (OtherComp :type Primitive%20Component%20Object%20Reference) (bSelfMoved :type Boolean) (HitLocation :type Vector :default "0, 0, 0") (HitNormal :type Vector :default "0, 0, 0") (NormalImpulse :type Vector :default "0, 0, 0") (Hit :type Hit%20Result%20Structure%20%28by%20ref%29))
  (bind _returnvalue (Game|GetPlayerCharacter 0))
  ;[0.05035 0.05035 0.05035] Destroy on hit
  (Utilities|IsValid _returnvalue
    (:Is%20Valid
      (Audio|PlaySoundatLocation "/Game/StarterContent/Audio/Explosion01.Explosion01" (Transformation|GetActorLocation _returnvalue) "0, 0, 0" 1.0 1.0 0.0 0 0 0 0)
      (Effects|SpawnEmitteratLocation "/Game/StarterContent/Particles/P_Explosion.P_Explosion" HitLocation "0, 0, 0" "5.000000,5.000000,5.000000")
      (bind (_outhits _returnvalue_2) (Collision|MultiSphereTraceForObjects HitLocation HitLocation (Variables|Default|GetExplosionRadius) (Utilities|Array|MakeArray "ObjectTypeQuery2") false 0 "None" false))
      (if _returnvalue_2
        (for _array_element _outhits
          (Game|Damage|ApplyDamage (.HitActor (Collision|BreakHitResult _array_element)) 1e+01 0 0)
          (if (Actor|ActorHasTag (.HitActor (Collision|BreakHitResult _array_element)) "Player")
            (Variables|Default|SetPlayerInRange true)))
        (Utilities|FlowControl|DoOnce false
          (:Completed
            (if (Variables|Default|GetPlayerInRange)
              (Character|LaunchCharacter (Game|GetPlayerCharacter 0) (* (Math|Vector|GetUnitDirection(Vector) HitLocation (Transformation|GetActorLocation (Game|GetPlayerCharacter 0))) (Variables|Default|GetLaunchDist)) false false))
            (Actor|DestroyActor)))
        (else
          (Actor|DestroyActor))))
    (:Is%20Not%20Valid
      (Actor|DestroyActor))))

(fn ConstructionScript)